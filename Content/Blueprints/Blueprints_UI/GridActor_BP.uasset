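; Grid actor that forwards the Fire input to its TileInteraction component as left mouse pointer presses and releases, for interacting with widgets.
; Its construction script calls a Construct event that is currently empty.
; A disconnected graph would fill GridLocations with GridX by GridY positions spaced by TileSize from the Tile component, creating a TileInteraction_W widget per cell, but it never runs.
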(event `Construct`)

(event `InputAction|Fire`
  (params (Key :type "Key Structure"))
  (:`Pressed`
    (`WidgetInteractionComponent.PressPointerKey` (`self.TileInteraction`) "LeftMouseButton"))
  (:`Released`
    (`WidgetInteractionComponent.ReleasePointerKey` (`self.TileInteraction`) "LeftMouseButton")))

(fn `UserConstructionScript`
  (`self.Construct`))