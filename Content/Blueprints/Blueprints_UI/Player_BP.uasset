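; Player Blueprint that holds a furniture inventory and seeds it with starting items at BeginPlay.
; InitializeInventory looks up hardcoded lava lamp and sofa rows in FurnitureTable_DT, appending each row to Inventory and a count to the parallel Instances array.
; The sofa lookup is chained to the lava lamp's Row Found output, so it only runs if that first row exists.
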(event `self.ReceiveBeginPlay`
  (`self.InitializeInventory`))

(fn `InitializeInventory`
  (bind _returnvalue (`|GetDataTableRow` "/Game/DataStructures/Tables/Tables_UI/FurnitureTable_DT.FurnitureTable_DT" "LavaLampItem")
    (:`then`
      (`KismetArrayLibrary.Array_Add` (`self.Inventory`) _returnvalue)
      (`KismetArrayLibrary.Array_Add` (`self.Instances`) 2)
      (bind _returnvalue_2 (`|GetDataTableRow` "/Game/DataStructures/Tables/Tables_UI/FurnitureTable_DT.FurnitureTable_DT" "Sofa")
        (:`then`
          (`KismetArrayLibrary.Array_Add` (`self.Inventory`) _returnvalue_2)
          (`KismetArrayLibrary.Array_Add` (`self.Instances`) 1))))))

(fn `UserConstructionScript`)