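; TileInteraction_BP is a grid actor of tile interaction widgets that hides itself in game at BeginPlay.
; The construction script builds a GridX by GridY array of rotated widget components spaced by TileSize, attached to the root, and records their relative locations.
; At BeginPlay it passes each component's world location to its TileInteraction_W widget as SpawnLocation, stopping if a cast fails.
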(event `self.ReceiveBeginPlay`
  (for _array_element (`self.GridComponents`)
    (bind _astile_interaction_w (cast `/Game/UI/UI_UI/TileInteraction_W` (`WidgetComponent.GetWidget` _array_element)))
    (set `/Game/UI/UI_UI/TileInteraction_W.SpawnLocation` (`SceneComponent.K2_GetComponentLocation` _array_element) _astile_interaction_w)
    (`self.SetActorHiddenInGame` true)))

(fn `UserConstructionScript`
  (bind _tilesize (`self.TileSize`))
  (`KismetArrayLibrary.Array_Clear` (`self.GridComponents`))
  (`KismetArrayLibrary.Array_Clear` (`self.GridLocations`))
  (for _index (range (`self.GridX`))
    (for _index_2 (range (`self.GridY`))
      (bind (_returnvalue_location _returnvalue_rotation _returnvalue_scale) (`KismetMathLibrary.BreakTransform` (`KismetMathLibrary.MakeTransform` (`KismetMathLibrary.MakeVector` (`KismetMathLibrary.Conv_IntToDouble` (* _index _tilesize)) (`KismetMathLibrary.Conv_IntToDouble` (* _index_2 _tilesize))) (struct :`Pitch` 90.0))))
      (bind _returnvalue (`AddComponent|NODE_AddWidgetComponent-1` :`bManualAttachment` true :`RelativeTransform` (`KismetMathLibrary.MakeTransform` _returnvalue_location _returnvalue_rotation _returnvalue_scale)))
      (`KismetArrayLibrary.Array_Add` (`self.GridComponents`) _returnvalue)
      (`KismetArrayLibrary.Array_Add` (`self.GridLocations`) _returnvalue_location)
      (`SceneComponent.K2_AttachToComponent` _returnvalue (`self.DefaultSceneRoot`) "None" "KeepRelative" "KeepRelative" "KeepRelative" true))))